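; GA_Fireball is a gameplay ability that has a UEFighterCharacter cast a fireball.
; On activation it plays the ability's montage, spawns BP_Fireball at the "Fire" notify, and ends when the montage completes.
; The fireball spawns just off the actor's location along the mesh's forward vector, with the character as owner and instigator.
; Hand socket locations are captured, but their midpoint calculation is unused.
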(event Ability|EventActivateAbility
  (bind _returnvalue (Ability|GetActorInfo))
  (bind _returnvalue_2 (Class|GASGameplayAbility|GetAbilityAnimation))
  (bind _asuefighter_character (Utilities|Casting|CastToUEFighterCharacter (.owneractor _returnvalue)))
  (Variables|Default|SetOwner _asuefighter_character)
  (Variables|Default|SetLeftHandLocation (Transformation|GetSocketLocation (.skeletalmeshcomponent _returnvalue) "LeftHandSocket"))
  (Variables|Default|SetRightHandLocation (Transformation|GetSocketLocation (.skeletalmeshcomponent _returnvalue) "RightHandSocket"))
  (Utilities|IsValid _returnvalue_2
    (:Is%20Valid
      (bind _notifyname (Animation|Montage|PlayMontage (.skeletalmeshcomponent _returnvalue) _returnvalue_2)
        (:OnCompleted
          (Ability|EndAbility))
        (:OnNotifyBegin
          (if (== _notifyname "Fire")
            (CallFunction|SpawnFireball)))))))

(fn SpawnFireball
  (bind _owner (Variables|Default|GetOwner))
  (bind _owner_2 (Variables|Default|GetOwner))
  (Game|SpawnActorfromClass "/Game/UEFighter/Blueprints/Abilities/BP_Fireball.BP_Fireball_C" (Math|Transform|MakeTransform (+ (Transformation|GetActorLocation _owner_2) (* (Math|Vector|GetForwardVector (Variables|/Script/Engine.Character|GetMesh _owner_2)) "1.000000,1.000000,1.000000")) (Transformation|GetActorRotation _owner) "1,1,1") "AlwaysSpawn" _owner _owner))